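; Spawner actor that periodically creates BP_Enemy actors around the player character.
; On BeginPlay it starts a looping timer that calls Spawn once per second.
; Spawn picks a random sign for X and Y and a random distance band on each axis, so enemies appear in the diagonal quadrants around the player, raised slightly, never right on top of them.
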(event Custom|Spawn
  ;[1 1 1] エネミースポーン
  (if (Math|Random|RandomBool)
    (Variables|Default|SetVar_X 1)
    (else
      (Variables|Default|SetVar_X -1)))
  (if (Math|Random|RandomBool)
    (Variables|Default|SetVar_Y 1)
    (else
      (Variables|Default|SetVar_Y -1)))
  (Game|SpawnActorfromClass "/Game/Blueprint/BP_Enemy.BP_Enemy_C" (Math|Conversions|ToTransform(Vector) (+ (Transformation|GetActorLocation (Game|GetPlayerCharacter 0)) (Math|Vector|MakeVector (* (Variables|Default|GetVar_X) (Math|Random|RandomFloatinRange 5e+02 1e+03)) (* (Variables|Default|GetVar_Y) (Math|Random|RandomFloatinRange 5e+02 1e+03)) 1e+02))) "Undefined" 0 0))

(event EventBeginPlay
  (Utilities|Time|SetTimerbyFunctionName 0 "Spawn" 1.0 true))

(fn ConstructionScript)