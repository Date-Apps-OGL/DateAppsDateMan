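; BP_Player is the player Blueprint that opens a transition selection screen when R is first pressed and applies yaw input through a CameraTurn event.
; The key press creates UI_Select, then spawns an indexed UI_Pointa pointer widget at each position in its PointaPos array.
; UI_TextAndButton is added last, with references wired so pointers and buttons reach UI_Select, which also references UI_TextAndButton.
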(event Custom|CameraTurn
  (params (Turn :type Float%20%28single-precision%29))
  (Pawn|Input|AddControllerYawInput Turn))

(event Input|KeyboardEvents|R
  (params (Key :type Key%20Structure :default "AnyKey"))
  ;[1 1 1] 移行画面表示
  (:Pressed
    (Utilities|FlowControl|DoOnce false
      (:Completed
        (bind _returnvalue (UserInterface|CreateWidget "/Game/UI_Select.UI_Select_C"))
        (UserInterface|Viewport|AddtoViewport _returnvalue 0) ; 選択画面を表示
        (for (_ _array_index) (Variables|/Game/UI_Select.UI_Select_C|GetPointaPos _returnvalue) ; 設定したPointaPosの数の分だけループ
          (bind _returnvalue_2 (UserInterface|CreateWidget "/Game/UI_Pointa.UI_Pointa_C")) ; ポインタを表示
          (Variables|/Game/UI_Pointa.UI_Pointa_C|SetArrayNumber _returnvalue_2 _array_index) ; 各ポインタに自分の添え字番号を設定
          (Class|Widget|SetRenderTranslation (Variables|/Game/UI_Pointa.UI_Pointa_C|GetPointaButton _returnvalue_2) (Utilities|Array|Get(acopy) (Variables|/Game/UI_Select.UI_Select_C|GetPointaPos _returnvalue) _array_index)) ; ポインタの位置指定
          (Variables|/Game/UI_Pointa.UI_Pointa_C|SetUI_Select _returnvalue_2 _returnvalue) ; 各ポインタがUI_Selectの情報を取得できるように
          (UserInterface|Viewport|AddtoViewport _returnvalue_2 0))
        (bind _returnvalue_3 (UserInterface|CreateWidget "/Game/UI_TextandButton.UI_TextAndButton_C")) ; ポインタを全てセットし終わったらボタン表示
        (bind _output_get (Variables|/Game/UI_TextandButton.UI_TextAndButton_C|SetUI_Select _returnvalue_3 _returnvalue)) ; UI_Selectの情報を取得できるように
        (bind _output_get_2 (Variables|/Game/UI_Select.UI_Select_C|SetUI_Text%20and%20Button _output_get _returnvalue_3)) ; UI_TextAndButtonの情報を取得できるようにように
        (UserInterface|Viewport|AddtoViewport _output_get_2 0)))))

(fn ConstructionScript)